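; Player controller for a Ping Pong game that handles the pause input.
; It caches the PingPongGamemode_BP reference on BeginPlay, and SetPause calls that game mode's PauseFun or ResumeFun based on IsPaused.
; Its own PauseFun and ResumeFun, not called here, manage the pause menu widget, input mode, cursor and game pause.
; Both store SetGamePaused's return value, a success flag, in IsPaused.
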(event `self.ReceiveBeginPlay`
  ; Set GameModeRef
  (bind _asping_pong_gamemode_bp (cast `/Game/Blueprints/PingPongGamemode_BP` (`GameplayStatics.GetGameMode`)))
  (set `self.GameModeRef` _asping_pong_gamemode_bp))

(event `InputAction|SetPause`
  (params (Key :type "Key Structure"))
  ; SetPause
  (:`Pressed`
    (if (`self.isPaused?`)
      (`/Game/Blueprints/PingPongGamemode_BP.ResumeFun` (`self.GameModeRef`))
      (else
        (`/Game/Blueprints/PingPongGamemode_BP.PauseFun` (`self.GameModeRef`))))))

(fn `PauseFun`
  (bind _returnvalue (`|CreateWidget` "/Game/Blueprints/PauseMenu_BW.PauseMenu_BW_C" (`GameplayStatics.GetPlayerController` 0)))
  (bind _output_get (set `self.PauseMenuRef` _returnvalue))
  (`UserWidget.AddToViewport` _output_get 0)
  (`WidgetBlueprintLibrary.SetInputMode_UIOnlyEx` (`GameplayStatics.GetPlayerController` 0) null)
  (bind _output_get_2 (set `self.bShowMouseCursor` true))
  (bind _returnvalue_2 (`GameplayStatics.SetGamePaused` _output_get_2))
  (set `self.IsPaused?` _returnvalue_2))

(fn `ResumeFun`
  (`Widget.RemoveFromParent` (`self.PauseMenuRef`))
  (`WidgetBlueprintLibrary.SetInputMode_GameOnly` (`GameplayStatics.GetPlayerController` 0))
  (bind _output_get (set `self.bShowMouseCursor` false))
  (bind _returnvalue (`GameplayStatics.SetGamePaused` _output_get))
  (set `self.IsPaused?` _returnvalue))

(fn `UserConstructionScript`)