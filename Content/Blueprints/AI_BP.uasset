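; AI opponent paddle that follows the ball along the X axis.
; On BeginPlay it reads the current difficulty from the game instance and sets its movement speed, faster on harder levels.
; Each tick, while the ball reference is valid, it moves toward the ball's X position at constant speed with a swept move, keeping its own Y and Z.
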(event `self.ReceiveTick`
  (params (DeltaSeconds :type "Float (single-precision)"))
  (bind (_returnvalue_x _returnvalue_y _returnvalue_z) (`KismetMathLibrary.BreakVector` (`self.K2_GetActorLocation`)))
  (bind _returnvalue_x_2 (`KismetMathLibrary.BreakVector` (`SceneComponent.K2_GetComponentLocation` (`/Game/Blueprints/Ball_BP.Sphere` (`self.BALLREF`)))))
  ; Paddle che segue la palla
  (`/Engine/EditorBlueprintResources/StandardMacros.IsValid` (`self.BALLREF`)
    (:`Is Valid`
      (`self.K2_SetActorLocation` (`KismetMathLibrary.VInterpTo_Constant` (`self.K2_GetActorLocation`) (`KismetMathLibrary.MakeVector` _returnvalue_x_2 _returnvalue_y _returnvalue_z) DeltaSeconds (`self.AI_SPEED`)) true))))

(event `self.ReceiveBeginPlay`
  ; Set Velocità a seconda della difficoltà
  (bind _asmy_game_istance_bp (cast `/Game/Blueprints/MyGameIstance_BP` (`GameplayStatics.GetGameInstance`)))
  (switch `/Game/Blueprints/E_Difficulty` (`/Game/Blueprints/MyGameIstance_BP.CurrentDifficulty` _asmy_game_istance_bp)
    (:`NewEnumerator0`
      (set `self.AI_SPEED` 300.0))
    (:`NewEnumerator1`
      (set `self.AI_SPEED` 600.0))
    (:`NewEnumerator2`
      (set `self.AI_SPEED` 900.0))))

(fn `UserConstructionScript`)