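; Game mode for a Ping Pong game that spawns the ball and handles pausing.
; On BeginPlay it finds the BallSpawn_BP actor and, after a short delay, spawns Ball_BP at its transform, re-finding the spawn point if the cached reference is invalid.
; Pause and resume events create or remove the pause menu widget, toggling game pause, input mode and mouse cursor.
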(event `self.ReceiveBeginPlay`
  ; Spawn della palla
  (bind _outactors (`GameplayStatics.GetAllActorsOfClass` "/Game/Blueprints/BallSpawn_BP.BallSpawn_BP_C"))
  (set `self.BallSpawnRef` (`|GetArrayItem` _outactors))
  (`KismetSystemLibrary.Delay` 0.2)
  (`self.SpawnBall`))

(event `SpawnBall`
  ; Spawn della palla
  (if (`KismetSystemLibrary.IsValid` (`self.BallSpawnRef`))
    (`|SpawnActorFromClass` "/Game/Blueprints/Ball_BP.Ball_BP_C" (`self.GetTransform` (`self.BallSpawnRef`)) "Undefined" "MultiplyWithRoot" null null)
    (else
      (bind _outactors (`GameplayStatics.GetAllActorsOfClass` "/Game/Blueprints/BallSpawn_BP.BallSpawn_BP_C"))
      (bind _output_get (set `self.BallSpawnRef` (`|GetArrayItem` _outactors)))
      (`|SpawnActorFromClass` "/Game/Blueprints/Ball_BP.Ball_BP_C" (`self.GetTransform` _output_get) "Undefined" "MultiplyWithRoot" null null))))

(event `PauseEvent`
  ; Eventi Per Pause
  (`self.PauseFun`))

(event `ResumeEvent`
  ; Eventi Per Pause
  (`self.ResumeFun`))

(fn `PauseFun`
  (bind _returnvalue (`|CreateWidget` "/Game/Blueprints/PauseMenu_BW.PauseMenu_BW_C" (`GameplayStatics.GetPlayerController` 0)))
  (bind _output_get (set `self.PauseMenuRef` _returnvalue))
  (`UserWidget.AddToViewport` _output_get 0)
  (`WidgetBlueprintLibrary.SetInputMode_UIOnlyEx` (`GameplayStatics.GetPlayerController` 0) null)
  (set `PlayerController.bShowMouseCursor` true (`GameplayStatics.GetPlayerController` 0))
  (bind _returnvalue_2 (`GameplayStatics.SetGamePaused` true))
  (set `self.isPaused?` _returnvalue_2))

(fn `ResumeFun`
  (`/Engine/EditorBlueprintResources/StandardMacros.IsValid` (`self.PauseMenuRef`)
    (:`Is Valid`
      (`Widget.RemoveFromParent` (`self.PauseMenuRef`))
      (`GameplayStatics.SetGamePaused` false)
      (`WidgetBlueprintLibrary.SetInputMode_GameOnly` (`GameplayStatics.GetPlayerController` 0))
      (set `PlayerController.bShowMouseCursor` false (`GameplayStatics.GetPlayerController` 0))
      (set `self.isPaused?` false))))

(fn `UserConstructionScript`)