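; Ball actor for a ping pong game that registers itself with the AI paddle and launches along Y on BeginPlay with a velocity impulse.
; Each hit plays a beep, raises the ball's speed and clamps its physics velocity to the new minimum.
; A near-zero Y velocity after a hit is pushed back up so the ball keeps crossing the court.
; When destroyed, it asks the game mode to spawn a replacement.
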(event `self.ReceiveBeginPlay`
  (bind _returnvalue (`GameplayStatics.GetActorOfClass` "/Game/Blueprints/AI_BP.AI_BP_C"))
  (bind _output_get (set `self.AI_REF` _returnvalue))
  (set `/Game/Blueprints/AI_BP.BALLREF` self _output_get)
  (`PrimitiveComponent.AddImpulse` (`self.Sphere`) (0.0 1000.0 0.0) "None" true))

(event `self.ReceiveHit`
  (params (MyComp :type "PrimitiveComponent Object Reference") (Other :type "Actor Object Reference") (OtherComp :type "PrimitiveComponent Object Reference") (bSelfMoved :type Boolean) (HitLocation :type "Vector Structure") (HitNormal :type "Vector Structure") (NormalImpulse :type "Vector Structure") (Hit :type "HitResult Structure (by ref)"))
  (`GameplayStatics.PlaySoundAtLocation` "/Game/Sounds/ping_pong_8bit_beeep__1_.ping_pong_8bit_beeep__1_" (`self.K2_GetActorLocation`) (struct) 1.0 1.0 0.0 null null null null)
  (set `self.BallSpeed` (+ (`self.BallSpeed`) 30.0))
  (bind _returnvalue (`PrimitiveComponent.GetPhysicsLinearVelocity` (`self.Sphere`) "None"))
  (`PrimitiveComponent.SetPhysicsLinearVelocity` (`self.Sphere`) (`KismetMathLibrary.ClampVectorSize` _returnvalue (`self.BallSpeed`) (`self.Max`)) false "None")
  (bind _returnvalue_2 (`PrimitiveComponent.GetPhysicsLinearVelocity` (`self.Sphere`) "None"))
  (if (<= (`KismetMathLibrary.Abs` (.y _returnvalue_2)) 50.0)
    (bind _returnvalue_3 (`PrimitiveComponent.GetPhysicsLinearVelocity` (`self.Sphere`) "None"))
    (`PrimitiveComponent.SetPhysicsLinearVelocity` (`self.Sphere`) (`KismetMathLibrary.MakeVector` (.x _returnvalue_3) (* (`KismetMathLibrary.SignOfFloat` (.y _returnvalue_3)) 300.0) (.z _returnvalue_3)) false "None")))

(event `self.ReceiveDestroyed`
  (bind _asping_pong_gamemode_bp (cast `/Game/Blueprints/PingPongGamemode_BP` (`GameplayStatics.GetGameMode`)))
  (`/Game/Blueprints/PingPongGamemode_BP.SpawnBall` _asping_pong_gamemode_bp))

(fn `UserConstructionScript`)